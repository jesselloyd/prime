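; Player-controlled Spike Monster hero character with world-axis movement, cursor aiming and a short blink.
; MoveUp and MoveRight add input along world X and Y, while holding right mouse makes Tick turn the control rotation toward the cursor's hit point.
; Space, gated by a cooldown flag and Delay, instantly shifts the capsule by half its velocity without a collision sweep.
; An unconnected debug line trace is left in the graph.
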(event Custom|FocusCharactersAttention
  (bind _returnvalue (Game|GetPlayerController 0))
  ;[1 1 1] Character rotation on click
  (Variables|Default|SetFocusCharBool true)
  (if (Variables|Default|GetFocusCharBool)
    (Pawn|SetControlRotation _returnvalue (Math|Conversions|RotationFromXVector (Math|Vector|Normalize (- (.Location (Collision|BreakHitResult (.HitResult (Game|Player|GetHitResultUnderCursorbyChannel _returnvalue "TraceTypeQuery2" true)))) (Transformation|GetActorLocation)))))))

(event Custom|BlurCharactersAttention
  ;[1 1 1] Character rotation on click
  (Variables|Default|SetFocusCharBool false))

(event EventTick
  (params (DeltaSeconds :type Float%20%28single-precision%29))
  (bind _returnvalue (Game|GetPlayerController 0))
  ;[1 1 1] Character rotation on click
  (if (Variables|Default|GetFocusCharBool)
    (Pawn|SetControlRotation _returnvalue (Math|Conversions|RotationFromXVector (Math|Vector|Normalize (- (.Location (Collision|BreakHitResult (.HitResult (Game|Player|GetHitResultUnderCursorbyChannel _returnvalue "TraceTypeQuery2" true)))) (Transformation|GetActorLocation)))))))

(event Collision|EventActorBeginOverlap
  (params (OtherActor :type Actor%20Object%20Reference)))

(event Input|AxisEvents|InputAxisMoveUp
  (params (AxisValue :type Float%20%28single-precision%29))
  ;[1 1 1] Movement
  (Pawn|Input|AddMovementInput "1.000000, 0, 0" AxisValue false))

(event Input|AxisEvents|InputAxisMoveRight
  (params (AxisValue :type Float%20%28single-precision%29))
  ;[1 1 1] Movement
  (Pawn|Input|AddMovementInput "0.000000,1.000000, 0" AxisValue false))

(event Input|MouseEvents|RightMouseButton
  (params (Key :type Key%20Structure :default "AnyKey"))
  (:Pressed
    (CallFunction|FocusCharactersAttention))
  (:Released
    (CallFunction|BlurCharactersAttention)))

(event Input|KeyboardEvents|SpaceBar
  (params (Key :type Key%20Structure :default "AnyKey"))
  (bind _capsulecomponent (Variables|Default|GetCapsuleComponent))
  (:Pressed
    (if (Variables|Default|GetcanJumpAgain)
      (Variables|Default|SetcanJumpAgain false)
      (Transformation|SetWorldLocation _capsulecomponent (+ (/ (Transformation|GetComponentVelocity _capsulecomponent) 2) (Transformation|GetActorLocation self)) false false)
      (Utilities|FlowControl|Delay 5.0)
      (Variables|Default|SetcanJumpAgain true))))

(fn ConstructionScript)